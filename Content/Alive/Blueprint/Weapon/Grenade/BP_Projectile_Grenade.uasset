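; BP_Projectile_Grenade is a grenade projectile that bursts on impact.
; On the first collision component hit against anything other than its instigator, it spawns a launcher impact particle effect at its location and sets a flag to block repeats.
; It then waits briefly before destroying itself, a delay the author notes as an unexplained workaround to keep the emitter working.
; The graph applies no damage.
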(event `self.ReceiveHit`
  (params (MyComp :type "PrimitiveComponent Object Reference") (Other :type "Actor Object Reference") (OtherComp :type "PrimitiveComponent Object Reference") (bSelfMoved :type Boolean) (HitLocation :type "Vector Structure") (HitNormal :type "Vector Structure") (NormalImpulse :type "Vector Structure") (Hit :type "HitResult Structure (by ref)")))

(event `self.CollisionComp.OnComponentHit`
  (params (HitComponent :type "PrimitiveComponent Object Reference") (OtherActor :type "Actor Object Reference") (OtherComp :type "PrimitiveComponent Object Reference") (NormalImpulse :type "Vector Structure") (Hit :type "HitResult Structure (by ref)"))
  (if (and (!= OtherActor (`self.GetInstigator`)) (not (`self.HasImpact`)))
    (`GameplayStatics.SpawnEmitterAtLocation` "/Game/ShooterGame/Effects/ParticleSystems/Weapons/RocketLauncher/Impact/P_Launcher_IH.P_Launcher_IH" (`self.K2_GetActorLocation`))
    (set `self.HasImpact` true)
    ;[1 1 1] TODO: I have no idea that the emitter doesn't work if not delay
    (`KismetSystemLibrary.Delay` 0.5)
    (`self.K2_DestroyActor`)))

(fn `UserConstructionScript`)