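; Bot character that equips a rifle and feeds combat stimuli to its AI blackboard.
; One second after BeginPlay it adds the weapon to its inventory and starts listening for ability-system attribute changes, which flag GetHurt.
; PawnSensing sets any seen BP_PlayerCharacter as AttackTarget.
; Retriggerable ten-second delays clear both keys, though sighting any pawn restarts the target timer.
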(event `self.ReceiveBeginPlay`
  (`KismetSystemLibrary.Delay` 1.0)
  (bind _returnvalue (`Weapon.NewWeapon` self "/Game/Alive/Blueprint/Weapon/Rifle/WT_Rifle_01.WT_Rifle_01_C" (`KismetMathLibrary.MakeTransform` (0.0 0.0 0.0))))
  (`WeaponInventoryComponent.AddWeaponToInventory` (`self.InventoryComponent`) _returnvalue)
  (`AttributeChanged.ListenForAttributeChange` (`self.AbilitySystemComponent`) (struct :`AttributeName` "Health" :`Attribute` "/Script/Alive.HealthSet:Health")
    (:`OnAttributeChanged`
      (`BlackboardComponent.SetValueAsBool` (`AIBlueprintHelperLibrary.GetBlackboard` (`self.GetController`)) "GetHurt" true)
      (`KismetSystemLibrary.RetriggerableDelay` 10.0)
      (`BlackboardComponent.SetValueAsBool` (`AIBlueprintHelperLibrary.GetBlackboard` (`self.GetController`)) "GetHurt" false))))

(event `self.PawnSensing.OnSeePawn`
  (params (Pawn :type "Pawn Object Reference"))
  (bind _returnvalue (`AIBlueprintHelperLibrary.GetBlackboard` (`self.GetController`)))
  (`|ExecutionSequence`
    (:`then_0`
      (bind _asbp_player_character (cast `/Game/Alive/Blueprint/Character/PlayerCharacter/BP_PlayerCharacter` Pawn))
      (`/Engine/EditorBlueprintResources/StandardMacros.IsValid` _returnvalue
        (:`Is Valid`
          (`BlackboardComponent.SetValueAsObject` _returnvalue "AttackTarget" _asbp_player_character))))
    (:`then_1`
      (`KismetSystemLibrary.RetriggerableDelay` 10.0)
      (`BlackboardComponent.SetValueAsObject` (`AIBlueprintHelperLibrary.GetBlackboard` (`self.GetController`)) "AttackTarget" null))))

(fn `UserConstructionScript`
  (`parent.UserConstructionScript`))