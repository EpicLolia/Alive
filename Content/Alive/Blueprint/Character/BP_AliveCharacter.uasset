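; BP_AliveCharacter is a player character with a rifle, sprinting, toggleable first-person and follow cameras, and a slow-motion toggle.
; Fire and reload input activate Gameplay Ability System abilities, with firing gated on and decrementing magazine ammo directly in the Blueprint.
; The Reload function refills the magazine from reserve ammo, and ammo changes trigger CallUpdateAmmo.
; It also creates the main screen widget for the local player and attaches the weapon to a hand socket.
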(event `self.ReceiveBeginPlay`
  (bind _returnvalue (`GameplayStatics.GetPlayerController` 0))
  (if (`Controller.IsLocalPlayerController` _returnvalue)
    (bind _returnvalue_2 (`|CreateWidget` "/Game/Alive/UI/WBP_MainScreen.WBP_MainScreen_C" _returnvalue))
    (`UserWidget.AddToViewport` _returnvalue_2 0)))

(event `Key|C`
  (params (Key :type "Key Structure"))
  (bind _followcamera (`self.FollowCamera`))
  (bind _firstpersoncameracomponent (`self.FirstPersonCameraComponent`))
  (:`Pressed`
    (`/Engine/EditorBlueprintResources/StandardMacros.FlipFlop`
      (:`A`
        (`ActorComponent.SetActive` _followcamera false false)
        (`ActorComponent.SetActive` _firstpersoncameracomponent true false))
      (:`B`
        (`ActorComponent.SetActive` _followcamera true false)
        (`ActorComponent.SetActive` _firstpersoncameracomponent false false)))))

(event `Key|Z`
  (params (Key :type "Key Structure"))
  (:`Pressed`
    (`/Engine/EditorBlueprintResources/StandardMacros.FlipFlop`
      (:`A`
        (`GameplayStatics.SetGlobalTimeDilation` 0.1))
      (:`B`
        (`GameplayStatics.SetGlobalTimeDilation` 1.0)))))

(event `Key|LeftMouseButton`
  (params (Key :type "Key Structure"))
  (:`Pressed`
    (if (> (`self.CurrentAmmo`) 0)
      (`AbilitySystemComponent.TryActivateAbilityByClass` (`AbilitySystemBlueprintLibrary.GetAbilitySystemComponent` self) "/Game/Alive/Blueprint/Character/Ability/GA_Rifle_FIre.GA_Rifle_FIre_C" true)
      (`GameplayStatics.PlaySoundAtLocation` "/Game/Alive/Audio/FirstPersonTemplateWeaponFire02.FirstPersonTemplateWeaponFire02" (`self.K2_GetActorLocation` self) (struct) 0.5 1.0 0.0 null null null)
      (`/Engine/EditorBlueprintResources/StandardMacros.DecrementInt` (`self.CurrentAmmo`)
        (:`  `
          (`self.UpdateAmmo`))))))

(event `InputAction|Sprint`
  (params (Key :type "Key Structure"))
  (bind _charactermovement (`self.CharacterMovement`))
  (:`Pressed`
    (set `CharacterMovementComponent.MaxWalkSpeed` 800.0 _charactermovement))
  (:`Released`
    (set `CharacterMovementComponent.MaxWalkSpeed` 500.0 _charactermovement)))

(event `InputAction|Reload`
  (params (Key :type "Key Structure"))
  (:`Pressed`
    (if (and (< (`self.CurrentAmmo`) (`self.MaxAmmoPerMagazine`)) (> (`self.RemainingAmmo`) 0))
      (`AbilitySystemComponent.TryActivateAbilityByClass` (`AbilitySystemBlueprintLibrary.GetAbilitySystemComponent` self) "/Game/Alive/Blueprint/Character/Ability/GA_Reload.GA_Reload_C" true))))

(fn `Reload`
  (if (>= (+ (`self.RemainingAmmo`) (`self.CurrentAmmo`)) (`self.MaxAmmoPerMagazine`))
    (set `self.RemainingAmmo` (- (`self.RemainingAmmo`) (- (`self.MaxAmmoPerMagazine`) (`self.CurrentAmmo`))))
    (set `self.CurrentAmmo` (`self.MaxAmmoPerMagazine`))
    (else
      (set `self.CurrentAmmo` (+ (`self.CurrentAmmo`) (`self.RemainingAmmo`)))
      (set `self.RemainingAmmo` 0)))
  (`self.UpdateAmmo`))

(fn `UserConstructionScript`
  (`SceneComponent.K2_AttachToComponent` (`self.Weapon`) (`self.Mesh`) "hand_r_wepSocket" "KeepRelative" "KeepRelative" "KeepRelative" true))