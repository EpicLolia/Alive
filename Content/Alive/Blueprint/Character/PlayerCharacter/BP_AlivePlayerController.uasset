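; Player controller for Alive that handles the local HUD, match history, floating damage numbers and leaving the room.
; Local controllers create the HUD with cursor input; Tab or ShowListOrRemove toggles a lazily created history list.
; Match results go to the game instance and are prepended to a history save slot.
; Damage events spawn parameterized Niagara numbers; leaving calls GoToEvaluateRoom, delayed on authority so clients exit first.
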(event `self.ReceiveBeginPlay`
  (if (`self.IsLocalPlayerController`)
    (set `self.bShowMouseCursor` true)
    (`WidgetBlueprintLibrary.SetInputMode_GameAndUIEx` self null)
    (bind _returnvalue (`|CreateWidget` "/Game/Alive/UI/InGame/WBP_ControllerHUD.WBP_ControllerHUD_C" self))
    (`UserWidget.AddToViewport` _returnvalue 0)))

(event `SaveGameLocally`
  (params (Ranking :type Integer) (Kills :type Integer) (Deaths :type Integer))
  (`self.LoadAndSaveGame` Ranking Kills Deaths))

(event `Key|Tab`
  (params (Key :type "Key Structure"))
  (bind _llistwidget (`self.LlistWidget`))
  ;[1 1 1] ShowList
  (:`Pressed`
    (`self.LlistWidget` :!label _label
      (:`then`
        _)
      (:`else`
        (bind _returnvalue (`|CreateWidget` "/Game/Alive/UI/MainMenu/WBP_HistoryList.WBP_HistoryList_C" self))
        (set `self.LlistWidget` _returnvalue)))
    (`/Engine/EditorBlueprintResources/StandardMacros.FlipFlop`
      (:`A`
        (`UserWidget.AddToViewport` _llistwidget 0)
        (`/Game/Alive/UI/MainMenu/WBP_HistoryList.ShowList` _llistwidget))
      (:`B`
        (`Widget.RemoveFromParent` _llistwidget)))))

(event `ShowListOrRemove`
  ;[1 1 1] ShowList
  (goto _label))

(event `LeaveRoom`
  (`/Engine/EditorBlueprintResources/ActorMacros.Switch Has Authority`
    (:`Authority`
      (`KismetSystemLibrary.Delay` 0.2) ; Wait Other Client to leave
    )
    (:`Remote`
      _))
  (bind _asbp_alive_game_instance (cast `/Game/Alive/Blueprint/BP_AliveGameInstance` (`GameplayStatics.GetGameInstance`)))
  (`/Game/Alive/Blueprint/BP_AliveGameInstance.GoToEvaluateRoom` _asbp_alive_game_instance))

(event `self.K2_OnCauseDamage`
  (params (DamageResult :type "DamageResult Structure (by ref)"))
  (bind (_oppositelocation _damage) (break `DamageResult` DamageResult))
  ;[1 1 1] Show Damage Number
  (bind _returnvalue (`NiagaraFunctionLibrary.SpawnSystemAtLocation` "/Game/Alive/Effect/Particle/NS_DamageNumber_Once.NS_DamageNumber_Once" _oppositelocation))
  (`self.SetDamageNumberParam` _returnvalue _damage))

(event `self.K2_OnSufferDamage`
  (params (DamageResult :type "DamageResult Structure (by ref)"))
  (bind _returnvalue (`self.K2_GetPawn`))
  ;[1 1 1] Show Damage Number
  (`/Engine/EditorBlueprintResources/StandardMacros.IsValid` _returnvalue
    (:`Is Valid`
      (bind _returnvalue_2 (`NiagaraFunctionLibrary.SpawnSystemAtLocation` "/Game/Alive/Effect/Particle/NS_DamageNumber_Once.NS_DamageNumber_Once" (`self.K2_GetActorLocation` _returnvalue)))
      (`self.SetDamageNumberParam` _returnvalue_2 (`.Damage` (break `DamageResult` DamageResult)) 1.0 12.0 (struct :`R` 0.009721 :`A` 1.0)))))

(fn `LoadAndSaveGame`
  (params (Ranking :type Integer) (Kills :type Integer) (Deaths :type Integer))
  (locals (SaveHistory :type "/Game/Alive/Blueprint/SaveGame/SaveGame_History Object Reference"))
  (bind _savehistory (`local.SaveHistory`))
  (bind _asbp_alive_game_instance (cast `/Game/Alive/Blueprint/BP_AliveGameInstance` (`GameplayStatics.GetGameInstance`)))
  (set `/Game/Alive/Blueprint/BP_AliveGameInstance.LastGameData` (make `/Game/Alive/Blueprint/SaveGame/SHistoryData` Ranking Kills Deaths (`KismetMathLibrary.Now`)) _asbp_alive_game_instance)
  (bind _returnvalue (`GameplayStatics.LoadGameFromSlot` "HistorySaveSlot"))
  (bind _assave_game_history (cast `/Game/Alive/Blueprint/SaveGame/SaveGame_History` _returnvalue)
    (:`then`
      (set `local.SaveHistory` _assave_game_history))
    (:`CastFailed`
      (bind _returnvalue_2 (`|GenericCreateObject` "/Game/Alive/Blueprint/SaveGame/SaveGame_History.SaveGame_History_C" self))
      (set `local.SaveHistory` _returnvalue_2)))
  (`KismetArrayLibrary.Array_Insert` (`/Game/Alive/Blueprint/SaveGame/SaveGame_History.ListData` (`local.SaveHistory`)) (make `/Game/Alive/Blueprint/SaveGame/SHistoryData` (`local.Ranking`) (`local.Kills`) (`local.Deaths`) (`KismetMathLibrary.Now`)))
  (`GameplayStatics.SaveGameToSlot` _savehistory (`/Game/Alive/Blueprint/SaveGame/SaveGame_History.SaveSlotName` _savehistory) (`/Game/Alive/Blueprint/SaveGame/SaveGame_History.UserIndex` _savehistory)))

(fn `SetDamageNumberParam`
  (params (TargetNS :type "NiagaraComponent Object Reference") (Damage :type "Float (double-precision)" :default 123456.0) (Duration :type "Float (double-precision)" :default 1.0) (SpriteSize :type "Float (double-precision)" :default 18.0) (Color :type "LinearColor Structure" :default (struct :`R` 0.07036 :`G` 0.171441 :`B` 0.165132 :`A` 1.0)))
  (`NiagaraComponent.SetVariableFloat` TargetNS "DamageNum" Damage)
  (`NiagaraComponent.SetVariableFloat` TargetNS "Duration" Duration)
  (`NiagaraComponent.SetVariableFloat` TargetNS "SpriteSize" SpriteSize)
  (`NiagaraComponent.SetVariableLinearColor` TargetNS "DamageNumColor" Color))

(fn `UserConstructionScript`)