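; BP_Spectator is a player spectator Blueprint that turns the view by touch drag.
; The first finger pressed while not rotating is stored with its start location and owns the rotation until that finger lifts.
; Each move of that finger adds controller yaw and pitch scaled from its offset to the initial press point, which is not updated during the drag.
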(event `InputTouch`
  (params (Location :type "Vector Structure") (FingerIndex :type "ETouchIndex Enum"))
  (bind (_prelocation_x _prelocation_y) (`KismetMathLibrary.BreakVector` (`self.PreLocation`)))
  (bind _returnvalue (and (`|EnumEquality` FingerIndex (`self.Finger Index`)) (`self.IsRotating`)))
  (:`Pressed`
    (if (not (`self.IsRotating`))
      (set `self.IsRotating` true)
      (set `self.Finger Index` FingerIndex)
      (set `self.PreLocation` Location)))
  (:`Released`
    (if _returnvalue
      (set `self.IsRotating` false)))
  (:`Moved`
    (if _returnvalue
      (`self.AddControllerYawInput` (* (- (.x Location) _prelocation_x) 0.05))
      (`self.AddControllerPitchInput` (* (- (.y Location) _prelocation_y) 0.05)))))

(fn `UserConstructionScript`)