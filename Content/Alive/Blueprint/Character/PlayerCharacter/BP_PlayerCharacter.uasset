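; Player character Blueprint that handles death presentation, weapon-change animation, item pickup and local UI.
; Death plays a random montage, then after a short random delay ragdolls with an impulse along the last movement velocity.
; Weapon changes always link the rifle anim layer and play the weapon's equip montage, while capsule overlaps try to collect pickups.
; Local possession creates mobile input and HUD widgets after a brief data-readiness delay, removed on EndPlay.
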(event `self.K2_OnDeathStarted`
  (bind _deathmontages (`self.DeathMontages`))
  ;[1 1 1] OnDeathStarted
  (`self.PlayAnimMontage` (`|GetArrayItem` _deathmontages (`KismetMathLibrary.RandomIntegerInRange` 0 (- (`KismetArrayLibrary.Array_Length` _deathmontages) 1))) 1.3)
  (`KismetSystemLibrary.Delay` (`KismetMathLibrary.RandomFloatInRange` 0.4 0.8))
  (`self.Ragdoll`))

(event `self.InventoryComponent.OnWeaponChanged`
  (params (Weapon :type "AliveWeapon Object Reference"))
  ;[1 1 1] Change Weapon And Anim
  (`SkeletalMeshComponent.LinkAnimClassLayers` (`self.Mesh`) "/Game/Alive/Character/Hero/Animations/Rifle/ABP_Layer_Rifle.ABP_Layer_Rifle_C")
  (`self.PlayAnimMontage` (`AliveWeapon.EquipMontage` Weapon)))

(event `self.ReceiveTick`
  (params (DeltaSeconds :type "Float (single-precision)"))
  ;[1 1 1] Tick For Debug
)

(event `self.K2_OnDeathFinished`
  ;[1 1 1] On Death Finish. Will destroy next frame
)

(event `self.CapsuleComponent.OnComponentBeginOverlap`
  (params (OverlappedComponent :type "PrimitiveComponent Object Reference") (OtherActor :type "Actor Object Reference") (OtherComp :type "PrimitiveComponent Object Reference") (OtherBodyIndex :type Integer) (bFromSweep :type Boolean) (SweepResult :type "HitResult Structure (by ref)"))
  ;[1 1 1] Try Pick Up Sth
  (bind _aspickup (cast `Pickup` OtherActor))
  (`Pickup.TryToPickItUp` _aspickup self))

(event `self.OnPossessedLocally`
  (params (LocalController :type "PlayerController Object Reference"))
  ;[1 1 1] Create Widget Locally
  ;;[1 0 0] Make sure that all player's data is ready!
  (`KismetSystemLibrary.Delay` 0.1)
  (`|ExecutionSequence`
    (:`then_0`
      (bind _returnvalue (`|CreateWidget` "/Game/Alive/UI/InGame/WBP_MoblieInput.WBP_MoblieInput_C" LocalController))
      (bind _output_get (set `self.InputWidget` _returnvalue))
      (`UserWidget.AddToViewport` _output_get 0))
    (:`then_1`
      (bind _returnvalue_2 (`|CreateWidget` "/Game/Alive/UI/InGame/WBP_CharacterHUD.WBP_CharacterHUD_C" LocalController))
      (bind _output_get_2 (set `self.HUD` _returnvalue_2))
      (`UserWidget.AddToViewport` _output_get_2 0))))

(event `self.ReceiveEndPlay`
  (params (EndPlayReason :type "EEndPlayReason Enum" :default "Destroyed"))
  ;[1 1 1] Remove widget
  (bind _inputwidget (`self.InputWidget`)
    (:`then`
      (`Widget.RemoveFromParent` _inputwidget))
    (:`else`
      _))
  (bind _hud (`self.HUD`)
    (:`then`
      (`Widget.RemoveFromParent` _hud))
    (:`else`)))

(fn `Ragdoll`
  (bind _ragdollimpulsebone (`self.RagdollImpulseBone`))
  (bind _mesh (`self.Mesh`))
  (bind _returnvalue (`CharacterMovementComponent.GetLastUpdateVelocity` (`self.CharacterMovement`)))
  ;[1 1 1] Activate Character Physics
  (`PrimitiveComponent.SetCollisionProfileName` _mesh "Ragdoll" true)
  (`SkeletalMeshComponent.SetAllBodiesBelowSimulatePhysics` _mesh _ragdollimpulsebone true true)
  (`PrimitiveComponent.AddImpulse` _mesh (+ _returnvalue (* (`KismetMathLibrary.Normal` _returnvalue) (`self.RagdollImpulseStrength`))) _ragdollimpulsebone true))

(fn `UserConstructionScript`)