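; Player character Blueprint with toggleable first-person and follow cameras, weapon animation and overlap pickups.
; Weapon changes always link the rifle anim layer and play that weapon's equip montage; BeginPlay adds mobile-input and main-screen widgets for the local player.
; Reload and grenade keys send tagged gameplay events to itself.
; Other keys toggle global slow motion and fire one lazily spawned, reused rifle projectile from the camera boom along base aim.
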(event `OnWeaponChanged_Event`
  (params (Weapon :type "AliveWeapon Object Reference"))
  (`SkeletalMeshComponent.LinkAnimClassLayers` (`self.Mesh`) "/Game/Alive/Character/Hero/Animations/Rifle/ABP_Layer_Rifle.ABP_Layer_Rifle_C")
  (`self.PlayAnimMontage` (`AliveWeapon.EquipMontage` Weapon)))

(event `self.ReceiveBeginPlay`
  (bind _returnvalue (`GameplayStatics.GetPlayerController` 0))
  (`|ExecutionSequence`
    (:`then_0`
      (add `AliveCharacter.OnWeaponChanged` (delegate `OnWeaponChanged_Event`)))
    (:`then_1`
      (if (`Controller.IsLocalPlayerController` _returnvalue)
        (bind _returnvalue_2 (`|CreateWidget` "/Game/Alive/UI/WBP_MoblieInput.WBP_MoblieInput_C" _returnvalue))
        (`UserWidget.AddToViewport` _returnvalue_2 0)
        (bind _returnvalue_3 (`|CreateWidget` "/Game/Alive/UI/WBP_MainScreen.WBP_MainScreen_C" _returnvalue))
        (`UserWidget.AddToViewport` _returnvalue_3 0)))))

(event `Key|R`
  (params (Key :type "Key Structure"))
  (:`Pressed`
    (`AbilitySystemBlueprintLibrary.SendGameplayEventToActor` self (struct :`TagName` "Data.AmmoReload"))))

(event `Key|X`
  (params (Key :type "Key Structure"))
  (bind _followcamera (`self.FollowCamera`))
  (bind _firstpersoncameracomponent (`self.FirstPersonCameraComponent`))
  (:`Pressed`
    (`/Engine/EditorBlueprintResources/StandardMacros.FlipFlop`
      (:`A`
        (`ActorComponent.SetActive` _followcamera false false)
        (`ActorComponent.SetActive` _firstpersoncameracomponent true false))
      (:`B`
        (`ActorComponent.SetActive` _followcamera true false)
        (`ActorComponent.SetActive` _firstpersoncameracomponent false false)))))

(event `Key|E`
  (params (Key :type "Key Structure"))
  (:`Pressed`
    (`AbilitySystemBlueprintLibrary.SendGameplayEventToActor` self (struct :`TagName` "Ability.Trigger.Weapon.Grenade"))))

(event `Key|Z`
  (params (Key :type "Key Structure"))
  (:`Pressed`
    (`/Engine/EditorBlueprintResources/StandardMacros.FlipFlop`
      (:`A`
        (`GameplayStatics.SetGlobalTimeDilation` 0.1))
      (:`B`
        (`GameplayStatics.SetGlobalTimeDilation` 1.0)))))

(event `Key|Q`
  (params (Key :type "Key Structure"))
  (:`Pressed`
    (`self.TraceProjectile`
      (:`then`
        _)
      (:`else`
        (bind _returnvalue (`|SpawnActorFromClass` "/Game/Alive/Blueprint/Weapon/Rifle/BP_Projectile_Rifle.BP_Projectile_Rifle_C" (`KismetMathLibrary.MakeTransform` (0.0 0.0 0.0)) "AlwaysSpawn" "OverrideRootScale" null 30 self))
        (bind _output_get (set `self.TraceProjectile` _returnvalue))))
    (`TraceProjectile.FireOnce` _output_get (`SceneComponent.K2_GetComponentLocation` (`self.CameraBoom`)) (`self.GetBaseAimRotation`) 1)))

(event `self.CapsuleComponent.OnComponentBeginOverlap`
  (params (OverlappedComponent :type "PrimitiveComponent Object Reference") (OtherActor :type "Actor Object Reference") (OtherComp :type "PrimitiveComponent Object Reference") (OtherBodyIndex :type Integer) (bFromSweep :type Boolean) (SweepResult :type "HitResult Structure (by ref)"))
  (bind _aspickup (cast `Pickup` OtherActor))
  (`Pickup.TryToPickItUp` _aspickup self))

(fn `UserConstructionScript`)