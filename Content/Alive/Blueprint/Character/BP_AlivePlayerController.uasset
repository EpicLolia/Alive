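; Player controller for the Alive game mode that manages the score list and the game-over screen.
; On BeginPlay it binds to the game state's game-over dispatcher, creates the score list widget and shows the cursor.
; Tab and the ShowListOrRemove event share a FlipFlop that toggles the list.
; Two seconds after game over, it switches to UI-only input and displays WBP_ConfigInfo with the elapsed time.
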(event `self.ReceiveBeginPlay`
  (bind _asbp_alive_game_state (cast `/Game/Alive/Blueprint/GameMode/BP_AliveGameState` (`GameplayStatics.GetGameState`)))
  (bind _output_get (set `self.Alive Game State` _asbp_alive_game_state))
  (add `/Game/Alive/Blueprint/GameMode/BP_AliveGameState.Dispatcher_GameOver` _output_get (delegate `CustomEvent_0`))
  (bind _returnvalue (`|CreateWidget` "/Game/Alive/UI/WBP_ScoreList.WBP_ScoreList_C" self))
  (set `self.LlistWidget` _returnvalue)
  (set `self.bShowMouseCursor` true))

(event `CustomEvent_0`
  (bind _returnvalue (`GameplayStatics.GetPlayerController` 0))
  (`KismetSystemLibrary.Delay` 2.0)
  (`WidgetBlueprintLibrary.SetInputMode_UIOnlyEx` _returnvalue null)
  (set `PlayerController.bShowMouseCursor` true _returnvalue)
  (bind _returnvalue_2 (`|CreateWidget` "/Game/Alive/UI/WBP_ConfigInfo.WBP_ConfigInfo_C" _returnvalue (`/Game/Alive/Blueprint/GameMode/BP_AliveGameState.Get Elapsed Time` (`self.Alive Game State`))))
  (`UserWidget.AddToViewport` _returnvalue_2 0))

(event `Key|Tab`
  (params (Key :type "Key Structure"))
  (bind _llistwidget (`self.LlistWidget`))
  (:`Pressed`
    (`/Engine/EditorBlueprintResources/StandardMacros.FlipFlop` :!label _label
      (:`A`
        (`UserWidget.AddToViewport` _llistwidget 0)
        (`/Game/Alive/UI/WBP_ScoreList.ShowList` _llistwidget))
      (:`B`
        (`Widget.RemoveFromParent` _llistwidget)))))

(event `ShowListOrRemove`
  (goto _label))

(fn `UserConstructionScript`)