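; BP_AliveGameMode is the game mode for Alive, which scatters score boxes at the start of a round.
; BeginPlay caches the BP_AliveGameState reference.
; GameStart spawns BP_Score_Box actors at random positions within a fixed volume, retrying until ten valid spawns exist because colliding placements can fail.
; It then passes the box count to the game state's own GameStart.
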(event `self.ReceiveBeginPlay`
  (bind _asbp_alive_game_state (cast `/Game/Alive/Blueprint/GameMode/BP_AliveGameState` (`GameplayStatics.GetGameState`)))
  (set `self.AliveGameState` _asbp_alive_game_state))

(fn `GameStart`
  (locals (Boxes :type Integer))
  (bind _boxes (`local.Boxes`))
  (while (< _boxes 10)
    (bind _returnvalue (`|SpawnActorFromClass` "/Game/Alive/Blueprint/Interaction/BP_Score_Box.BP_Score_Box_C" (`KismetMathLibrary.MakeTransform` (`KismetMathLibrary.MakeVector` (`KismetMathLibrary.RandomFloatInRange` -1600.0 1600.0) (`KismetMathLibrary.RandomFloatInRange` -1600.0 1600.0) (`KismetMathLibrary.RandomFloatInRange` 200.0 400.0))) "AdjustIfPossibleButDontSpawnIfColliding" "OverrideRootScale" null null))
    (`/Engine/EditorBlueprintResources/StandardMacros.IsValid` _returnvalue
      (:`Is Valid`
        (`/Engine/EditorBlueprintResources/StandardMacros.IncrementInt` (`local.Boxes`)))))
  (`/Game/Alive/Blueprint/GameMode/BP_AliveGameState.GameStart` (`self.AliveGameState`) _boxes))

(fn `UserConstructionScript`)