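; Game state for the Alive game mode that tracks a timed box-hitting round from start to game over.
; GameStart stores the box count and fires a start dispatcher, then waits briefly before marking the game active and stamping the start time.
; HitOneBox decrements the count, signals the update and, at zero, stamps the end time and fires game over.
; Elapsed time uses server world time, freezing once the round ends.
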(event `GameStart`
  (params (RemaingBoxes :type Integer))
  (set `self.RemaingBoxes` RemaingBoxes)
  (`self.Dispatcher_GameStart`)
  (`KismetSystemLibrary.Delay` 3.0)
  (set `self.InGame` true)
  (set `self.BeginTimestamp` (`self.GetServerWorldTimeSeconds`)))

(fn `Get Elapsed Time`
  (returns (ElapsedTime :type "Float (double-precision)"))
  (if (`self.InGame`)
    (return (- (`self.GetServerWorldTimeSeconds`) (`self.BeginTimestamp`)))
    (else
      (return (- (`self.EndTimestamp`) (`self.BeginTimestamp`))))))

(fn `HitOneBox`
  (bind _result (`/Engine/EditorBlueprintResources/StandardMacros.DecrementInt` (`self.RemaingBoxes`))
    (:`  `
      (`self.UpdateRemainingBoxes`)
      (if (== _result 0)
        (set `self.InGame` false)
        (set `self.EndTimestamp` (`self.GetServerWorldTimeSeconds`))
        (`self.Dispatcher_GameOver`)))))

(fn `UserConstructionScript`)