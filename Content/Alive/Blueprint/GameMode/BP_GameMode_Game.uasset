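; Match game mode for Alive that drives player spawning, result saving and leaving from the game state's match state changes.
; On Playing it swaps each player's spectator pawn for a character; players logging in mid-match spawn immediately.
; On Finish it ranks players by kills minus deaths and has each controller save rank, kills and deaths locally.
; On Evaluate it tells every player controller to leave the room.
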(event `self.ReceiveBeginPlay`
  (`self.AliveGameState`
    (:`then`
      _)
    (:`else`
      (bind _asbp_alive_game_state (cast `/Game/Alive/Blueprint/GameMode/BP_AliveGameState` (`GameplayStatics.GetGameState`)))
      (set `self.AliveGameState` _asbp_alive_game_state)))
  (add `AliveGameState.OnMatchStateChanged` (`self.AliveGameState`) (delegate `OnMatchStateChanged_Event`)))

(event `OnMatchStateChanged_Event`
  (params (CurrentMatchState :type "EMatchState Enum" :default "Warmup"))
  (switch `EMatchState` CurrentMatchState
    (:`Playing`
      (`self.SpawnAllPlayers`))
    (:`Finish`
      (`self.CallAllPlayersToSaveGame`))
    (:`Evaluate`
      (`self.CallAllPlayersToLeave`))))

(event `self.K2_PostLogin`
  (params (NewPlayer :type "PlayerController Object Reference"))
  ;[1 1 1] Spawn directly if game has started
  (`self.AliveGameState`
    (:`then`
      _)
    (:`else`
      (bind _asbp_alive_game_state (cast `/Game/Alive/Blueprint/GameMode/BP_AliveGameState` (`GameplayStatics.GetGameState`)))
      (set `self.AliveGameState` _asbp_alive_game_state)))
  (if (`|EnumEquality` (`AliveGameState.MatchState` (`self.AliveGameState`)) "Playing")
    (bind _asbp_alive_player_controller (cast `/Game/Alive/Blueprint/Character/PlayerCharacter/BP_AlivePlayerController` NewPlayer))
    (`AlivePlayerController.SpawnPlayerCharacterImmediately` _asbp_alive_player_controller)))

(fn `CallAllPlayersToLeave`
  (for _array_element (`GameStateBase.PlayerArray` (`self.AliveGameState`))
    (bind _asbp_alive_player_controller (cast `/Game/Alive/Blueprint/Character/PlayerCharacter/BP_AlivePlayerController` (`self.GetOwner` _array_element)))
    (`/Game/Alive/Blueprint/Character/PlayerCharacter/BP_AlivePlayerController.LeaveRoom` _asbp_alive_player_controller)))

(fn `CallAllPlayersToSaveGame`
  (locals (CurrentRanking :type Integer) (CurrentPlayer :type "/Game/Alive/Blueprint/Character/PlayerCharacter/BP_AlivePlayerState Object Reference"))
  (bind _currentplayer (`local.CurrentPlayer`))
  (bind _currentplayer_2 (`local.CurrentPlayer`))
  (for _array_element (`GameStateBase.PlayerArray` (`self.AliveGameState`))
    (bind _asbp_alive_player_state (cast `/Game/Alive/Blueprint/Character/PlayerCharacter/BP_AlivePlayerState` _array_element))
    (set `local.CurrentPlayer` _asbp_alive_player_state)
    ;[1 1 1] Calculate Ranking
    (set `local.CurrentRanking` 1)
    (for _array_element_2 (`GameStateBase.PlayerArray` (`self.AliveGameState`))
      (bind _asbp_alive_player_state_2 (cast `/Game/Alive/Blueprint/Character/PlayerCharacter/BP_AlivePlayerState` _array_element_2))
      (if (> (- (`AlivePlayerState.KillCount` _asbp_alive_player_state_2) (`AlivePlayerState.DeathCount` _asbp_alive_player_state_2)) (- (`AlivePlayerState.KillCount` _currentplayer_2) (`AlivePlayerState.DeathCount` _currentplayer_2)))
        (`/Engine/EditorBlueprintResources/StandardMacros.IncrementInt` (`local.CurrentRanking`))))
    ;[1 1 1] SaveGame
    (bind _asbp_alive_player_controller (cast `/Game/Alive/Blueprint/Character/PlayerCharacter/BP_AlivePlayerController` (`self.GetOwner` (`local.CurrentPlayer`))))
    (`/Game/Alive/Blueprint/Character/PlayerCharacter/BP_AlivePlayerController.SaveGameLocally` _asbp_alive_player_controller (`local.CurrentRanking`) (`AlivePlayerState.KillCount` _currentplayer) (`AlivePlayerState.DeathCount` _currentplayer))))

(fn `SpawnAllPlayers`
  (locals (CurrentController :type "AlivePlayerController Object Reference"))
  (for _array_element (`GameStateBase.PlayerArray` (`self.AliveGameState`))
    (bind _asalive_player_controller (cast `AlivePlayerController` (`self.GetOwner` _array_element)))
    (set `local.CurrentController` _asalive_player_controller)
    (bind _returnvalue (`Controller.K2_GetPawn` _asalive_player_controller))
    ;[1 1 1] Remove the Spectator Pawn
    (`/Engine/EditorBlueprintResources/StandardMacros.IsValid` _returnvalue
      (:`Is Valid`
        (`self.SetLifeSpan` _returnvalue 0.1)
        (`Controller.UnPossess` (`local.CurrentController`)))
      (:`Is Not Valid`
        _))
    (`AlivePlayerController.SpawnPlayerCharacterImmediately` (`local.CurrentController`))))

(fn `UserConstructionScript`)