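; BP_Score_Box is a box actor that scores once when a player hits it during a match.
; On HittedByPlayer it checks that the Alive game state is in game and the box is unhit, then calls HitOneBox on that state.
; It then sets a hit flag, turns on physics simulation for its static mesh and destroys itself after a short delay.
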(event `HittedByPlayer`
  (params (Instigator :type "Actor Object Reference"))
  (bind _asbp_alive_game_state (cast `/Game/Alive/Blueprint/GameMode/BP_AliveGameState` (`GameplayStatics.GetGameState`)))
  (if (and (`/Game/Alive/Blueprint/GameMode/BP_AliveGameState.InGame` _asbp_alive_game_state) (not (`self.HasHit`)))
    (`/Game/Alive/Blueprint/GameMode/BP_AliveGameState.HitOneBox` _asbp_alive_game_state)
    (set `self.HasHit` true)
    (`PrimitiveComponent.SetSimulatePhysics` (`self.StaticMesh`) true)
    (`KismetSystemLibrary.Delay` 0.5)
    (`self.K2_DestroyActor`)))

(fn `UserConstructionScript`)