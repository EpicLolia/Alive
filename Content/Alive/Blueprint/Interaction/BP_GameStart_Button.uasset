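; BP_GameStart_Button is a shootable in-world button that starts a round of the Alive game.
; A hit from a FirstPersonProjectile calls GameStart on BP_AliveGameMode, then hides the mesh and disables its collision.
; On BeginPlay it caches the game mode and binds to the game state's GameOver dispatcher, which restores the button's visibility and collision.
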(event `self.ReceiveBeginPlay`
  (bind _asbp_alive_game_mode (cast `/Game/Alive/Blueprint/GameMode/BP_AliveGameMode` (`GameplayStatics.GetGameMode`)))
  (set `self.Alive Game Mode` _asbp_alive_game_mode)
  (bind _asbp_alive_game_state (cast `/Game/Alive/Blueprint/GameMode/BP_AliveGameState` (`GameplayStatics.GetGameState`)))
  (add `/Game/Alive/Blueprint/GameMode/BP_AliveGameState.Dispatcher_GameOver` _asbp_alive_game_state (delegate `GameOver`)))

(event `GameOver`
  (bind _staticmesh (`self.StaticMesh`))
  (`SceneComponent.SetVisibility` _staticmesh true false)
  (`PrimitiveComponent.SetCollisionEnabled` _staticmesh "QueryAndPhysics"))

(event `self.StaticMesh.OnComponentHit`
  (params (HitComponent :type "PrimitiveComponent Object Reference") (OtherActor :type "Actor Object Reference") (OtherComp :type "PrimitiveComponent Object Reference") (NormalImpulse :type "Vector Structure") (Hit :type "HitResult Structure (by ref)"))
  (bind _staticmesh (`self.StaticMesh`))
  (cast `/Game/Alive/Weapon/Projectile/Yellow/FirstPersonProjectile` OtherActor)
  (`/Game/Alive/Blueprint/GameMode/BP_AliveGameMode.GameStart` (`self.Alive Game Mode`))
  (`SceneComponent.SetVisibility` _staticmesh false false)
  (`PrimitiveComponent.SetCollisionEnabled` _staticmesh "NoCollision"))

(fn `UserConstructionScript`)