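; Animation modifier that automatically places left and right foot sync markers on an animation sequence.
; On apply, it adds a notify track and scans every frame of both foot IK bones.
; A marker lands where bone height is lower than both adjacent frames and higher two frames before than two frames after.
; On revert, it removes that notify track.
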(event `self.OnApply`
  (params (AnimationSequence :type "AnimSequence Object Reference"))
  (bind _output_get (set `self.Animation Sequence` AnimationSequence))
  (`AnimationBlueprintLibrary.AddAnimationNotifyTrack` _output_get (`self.NotifyTrackName`))
  (for _index (range (+ (`AnimationBlueprintLibrary.GetNumFrames` (`self.Animation Sequence`)) 1))
    (`|ExecutionSequence`
      (:`then_0`
        (`self.SetFootSyncMarker` _index (`self.LeftFootMarkerName`) (`self.NotifyTrackName`) (`self.LeftFootIK_Bone`)))
      (:`then_1`
        (`self.SetFootSyncMarker` _index (`self.RightFootMarkerName`) (`self.NotifyTrackName`) (`self.RightFootIK_Bone`)))))
  (`AnimationBlueprintLibrary.FinalizeBoneAnimation` (`self.Animation Sequence`)))

(event `self.OnRevert`
  (params (AnimationSequence :type "AnimSequence Object Reference"))
  (bind _output_get (set `self.Animation Sequence` AnimationSequence))
  (`AnimationBlueprintLibrary.RemoveAnimationNotifyTrack` _output_get (`self.NotifyTrackName`)))

(fn `SetFootSyncMarker`
  (params (Frame :type Integer) (MarkerName :type Name) (NotifyTrackName :type Name) (IK_BoneName :type Name))
  (bind _animation_sequence (`self.Animation Sequence`))
  (bind _pose (`AnimationBlueprintLibrary.GetBonePoseForFrame` _animation_sequence IK_BoneName Frame))
  (if (and (and (< (.z (.location _pose)) (.z (.location (`AnimationBlueprintLibrary.GetBonePoseForFrame` _animation_sequence IK_BoneName (- Frame 1))))) (< (.z (.location _pose)) (.z (.location (`AnimationBlueprintLibrary.GetBonePoseForFrame` _animation_sequence IK_BoneName (+ Frame 1)))))) (> (.z (.location (`AnimationBlueprintLibrary.GetBonePoseForFrame` _animation_sequence IK_BoneName (- Frame 2)))) (.z (.location (`AnimationBlueprintLibrary.GetBonePoseForFrame` _animation_sequence IK_BoneName (+ Frame 2))))))
    (`AnimationBlueprintLibrary.AddAnimationSyncMarker` (`self.Animation Sequence`) MarkerName (`AnimationBlueprintLibrary.GetTimeAtFrame` (`self.Animation Sequence`) Frame) NotifyTrackName)))